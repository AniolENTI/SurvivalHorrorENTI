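; BP_Zombi is a zombie Blueprint that takes damage and explodes when killed.
; BeginPlay sets Health to 100, and the TakeDamage event subtracts the incoming amount, calling Die at zero or below.
; Die spawns an explosion particle at the actor's location, then destroys the actor.
; The graph holds no movement, AI or attack logic.
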(event `self.ReceiveBeginPlay`
  (set `self.Health` 100.0))

(event `self.TakeDamage`
  (params (Amount :type "Float (double-precision)"))
  (set `self.Health` (- (`self.Health`) Amount))
  (if (<= (`self.Health`) 0.0)
    (`self.Die`)))

(event `self.Die`
  (`GameplayStatics.SpawnEmitterAtLocation` "/Game/StarterContent/Particles/P_Explosion.P_Explosion" (`self.K2_GetActorLocation`))
  (`self.K2_DestroyActor`))

(fn `UserConstructionScript`)